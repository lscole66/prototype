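; Base map marker actor for the guidance system, showing a sprite icon and an in-world indicator widget from one texture.
; After a short BeginPlay delay, a server-to-multicast call registers it as a point of interest with the nearest BP_MapBoundaries.
; Overlap triggers react only to actors with BPC_MasterGuidance.
; One optionally has that component remove the marker on touch; the other toggles widget visibility unless it is always displayed.
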(event `self.ReceiveBeginPlay`
  ;[1 1 1] Wait 2 second to call the get boundaries on the server
  (`KismetSystemLibrary.Delay` 1.0)
  (`self.GetBoundarieRef_server`)
  (bind _aswbp_in_world_indication (cast `/Game/MasterRpgFramework/MasterGuidanceSystem/RadarSystem/WIdgets/WBP_InWorldIndication` (`WidgetComponent.GetWidget` (`self.Widget`))))
  (`/Game/MasterRpgFramework/MasterGuidanceSystem/RadarSystem/WIdgets/WBP_InWorldIndication.StartWIdget` _aswbp_in_world_indication (`self.Map MarkerTexture`)))

(event `GetBoundarieRef_server`
  ;[1 1 1] Get the map boundarie overlap this actor
  (`self.GetBoundarieRef_multicast`))

(event `GetBoundarieRef_multicast`
  ;[1 1 1] Get the map boundarie overlap this actor
  (bind _outactors (`GameplayStatics.GetAllActorsOfClass` "/Game/MasterRpgFramework/MasterGuidanceSystem/Blueprints/MapBoundaries/BP_MapBoundaries.BP_MapBoundaries_C"))
  (bind (_distance _returnvalue) (`GameplayStatics.FindNearestActor` (`self.K2_GetActorLocation` self) _outactors))
  (`/Engine/EditorBlueprintResources/StandardMacros.IsValid` _returnvalue
    (:`Is Valid`
      (bind _boundariereturn (message `/Game/MasterRpgFramework/MasterGuidanceSystem/Blueprints/MapBoundaries/BPI_MapBoundaries.I_ReturnBoundarieRef` _returnvalue))
      (bind _output_get (set `self.MapBoundarieRef` _boundariereturn))
      (`KismetArrayLibrary.Array_AddUnique` (`/Game/MasterRpgFramework/MasterGuidanceSystem/Blueprints/MapBoundaries/BP_MapBoundaries.MapPointsOfInterest` _output_get) self))))

(event `self.RemoveMarkerTrigger.OnComponentBeginOverlap`
  (params (OverlappedComponent :type "PrimitiveComponent Object Reference") (OtherActor :type "Actor Object Reference") (OtherComp :type "PrimitiveComponent Object Reference") (OtherBodyIndex :type Integer) (bFromSweep :type Boolean) (SweepResult :type "HitResult Structure (by ref)"))
  (bind _returnvalue (`self.GetComponentByClass` OtherActor "/Game/MasterRpgFramework/MasterGuidanceSystem/Components/BPC_MasterGuidance.BPC_MasterGuidance_C"))
  ;[1 1 1] On Actor enter check if have the valid map component if yes we can remove this marker
  (`/Engine/EditorBlueprintResources/StandardMacros.IsValid` _returnvalue
    (:`Is Valid`
      (if (`self.DestoryOnTouch`)
        (`/Game/MasterRpgFramework/MasterGuidanceSystem/Components/BPC_MasterGuidance.RemovePlayerMarker` _returnvalue self)))))

(event `self.ToogleWidget.OnComponentBeginOverlap`
  (params (OverlappedComponent :type "PrimitiveComponent Object Reference") (OtherActor :type "Actor Object Reference") (OtherComp :type "PrimitiveComponent Object Reference") (OtherBodyIndex :type Integer) (bFromSweep :type Boolean) (SweepResult :type "HitResult Structure (by ref)"))
  ;[1 1 1] Toogle the in work widget
  (if (not (`self.Always Display Widget`))
    (`/Engine/EditorBlueprintResources/StandardMacros.IsValid` (`self.GetComponentByClass` OtherActor "/Game/MasterRpgFramework/MasterGuidanceSystem/Components/BPC_MasterGuidance.BPC_MasterGuidance_C")
      (:`Is Valid`
        (`SceneComponent.SetVisibility` (`self.Widget`) true false)))))

(event `self.ToogleWidget.OnComponentEndOverlap`
  (params (OverlappedComponent :type "PrimitiveComponent Object Reference") (OtherActor :type "Actor Object Reference") (OtherComp :type "PrimitiveComponent Object Reference") (OtherBodyIndex :type Integer))
  ;[1 1 1] Toogle the in work widget
  (if (not (`self.Always Display Widget`))
    (`/Engine/EditorBlueprintResources/StandardMacros.IsValid` (`self.GetComponentByClass` OtherActor "/Game/MasterRpgFramework/MasterGuidanceSystem/Components/BPC_MasterGuidance.BPC_MasterGuidance_C")
      (:`Is Valid`
        (`SceneComponent.SetVisibility` (`self.Widget`) false false)))))

(fn `UserConstructionScript`
  (bind _map_markertexture (`self.Map MarkerTexture`))
  (`/Engine/EditorBlueprintResources/StandardMacros.IsValid` _map_markertexture
    (:`Is Valid`
      (`BillboardComponent.SetSprite` (`self.IconDisplayPosition`) _map_markertexture))))