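; BP_FogOfWar is a placeable fog-of-war area that is discovered when an actor with a BPC_MasterGuidance component reaches it.
; The construction script sizes the area sphere from AreaRadius and the discovery sphere from that radius plus an additional margin.
; Overlapping the discovery sphere reports the area once to that component via OnDiscoverArea.
; OnDiscovered, meant to fire after the component registers the discovery, destroys the actor.
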(event `self.DiscoverSphere.OnComponentBeginOverlap`
  (params (OverlappedComponent :type "PrimitiveComponent Object Reference") (OtherActor :type "Actor Object Reference") (OtherComp :type "PrimitiveComponent Object Reference") (OtherBodyIndex :type Integer) (bFromSweep :type Boolean) (SweepResult :type "HitResult Structure (by ref)"))
  (bind _returnvalue (`self.GetComponentByClass` OtherActor "/Game/MasterRpgFramework/MasterGuidanceSystem/Components/BPC_MasterGuidance.BPC_MasterGuidance_C"))
  ;[0 1 0.08199] On the object that have the component touch this will trigget the undiscover the area
  (`/Engine/EditorBlueprintResources/StandardMacros.IsValid` _returnvalue
    (:`Is Valid`
      (`/Engine/EditorBlueprintResources/StandardMacros.DoOnce` false
        (:`Completed`
          (`/Game/MasterRpgFramework/MasterGuidanceSystem/Components/BPC_MasterGuidance.OnDiscoverArea` _returnvalue self))))))

(event `OnDiscovered`
  ;[1 0.08006 0] This is trigger after the bpc register the event
  (`self.K2_DestroyActor`))

(fn `UserConstructionScript`
  (bind _arearadius (`self.AreaRadius`))
  (`SphereComponent.SetSphereRadius` (`self.AreaShepere`) _arearadius false)
  (`SphereComponent.SetSphereRadius` (`self.DiscoverSphere`) (+ _arearadius (`self.AddicionalDiscoverRadius`)) false))