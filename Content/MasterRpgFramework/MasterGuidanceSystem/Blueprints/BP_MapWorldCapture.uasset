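; BP_MapWorldCapture is an editor-placed actor that captures the world between two map corners to a texture intended for building a map.
; Its construction script centers the actor in X and Y between the MapBoundaries corner actors, keeping its own height.
; It sets the SceneCapture ortho width to the larger X or Y span, printing a warning if references are missing.
; The event graph has no runtime logic.
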(fn `UserConstructionScript`
  (bind (_returnvalue_x _returnvalue_y _returnvalue_z) (`KismetMathLibrary.BreakVector` (`self.K2_GetActorLocation`)))
  (bind _mapboundaries (`self.MapBoundaries`))
  (bind _mapboundaries_2 (`self.MapBoundaries`))
  (bind _mapboundaries_3 (`self.MapBoundaries`))
  (bind _returnvalue (`self.K2_GetActorLocation` (`/Game/MasterRpgFramework/MasterGuidanceSystem/Blueprints/MapBoundaries/BP_MapBoundaries.UpperRightCorner` _mapboundaries_2)))
  (bind (_returnvalue_x_2 _returnvalue_y_2) (`KismetMathLibrary.BreakVector` (`self.K2_GetActorLocation` (`/Game/MasterRpgFramework/MasterGuidanceSystem/Blueprints/MapBoundaries/BP_MapBoundaries.UpperRightCorner` _mapboundaries_3))))
  (bind (_returnvalue_x_3 _returnvalue_y_3) (`KismetMathLibrary.BreakVector` (`self.K2_GetActorLocation` (`/Game/MasterRpgFramework/MasterGuidanceSystem/Blueprints/MapBoundaries/BP_MapBoundaries.LowerLeftCorner` _mapboundaries_3))))
  (`/Engine/EditorBlueprintResources/StandardMacros.IsValid` (`self.MapBoundaries`)
    (:`Is Valid`
      ;[1 1 1] This Actor is goin to capture a scene betweet two target points and output a texture so we can save this texture and use to create a map in the future
      ;;[1 1 1] Make sure the upper left conner and lower right conner is valid
      (if (and (`KismetSystemLibrary.IsValid` (`/Game/MasterRpgFramework/MasterGuidanceSystem/Blueprints/MapBoundaries/BP_MapBoundaries.UpperRightCorner` _mapboundaries)) (`KismetSystemLibrary.IsValid` (`/Game/MasterRpgFramework/MasterGuidanceSystem/Blueprints/MapBoundaries/BP_MapBoundaries.LowerLeftCorner` _mapboundaries)))
        (`self.K2_SetActorLocation` (`KismetMathLibrary.MakeVector` (.x (+ _returnvalue (/ (- (`self.K2_GetActorLocation` (`/Game/MasterRpgFramework/MasterGuidanceSystem/Blueprints/MapBoundaries/BP_MapBoundaries.LowerLeftCorner` _mapboundaries_2)) _returnvalue) 2.0))) (.y (+ _returnvalue (/ (- (`self.K2_GetActorLocation` (`/Game/MasterRpgFramework/MasterGuidanceSystem/Blueprints/MapBoundaries/BP_MapBoundaries.LowerLeftCorner` _mapboundaries_2)) _returnvalue) 2.0))) _returnvalue_z) false true)
        ;;[1 1 1] Put the capture in the texture with the right size
        (set `SceneCaptureComponent2D.OrthoWidth` (`KismetMathLibrary.FMax` (`KismetMathLibrary.Abs` (- _returnvalue_x_3 _returnvalue_x_2)) (`KismetMathLibrary.Abs` (- _returnvalue_y_3 _returnvalue_y_2))) (`self.SceneCapture`))
        (else
          (`KismetSystemLibrary.PrintString` "Please Setup the upper left corner and Lower right corner"))))
    (:`Is Not Valid`
      (`KismetSystemLibrary.PrintString` "Please Setup the map Boundaries you wnat to render the image"))))