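; Save game object for the RPG inventory framework that stores player progress: items, recipes, slots, currency, cooldowns, quests, tutorials, attributes, talents and input mappings.
; SaveData flattens action and bag slots to item data, and chest and vendor actors to structs of transform, inventory, ID and class.
; It also records the save name and a timestamp.
; LoadData returns the stored gameplay data, and FNGameSaveImage builds the save's PNG path.
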(fn `FN_GameSaveImage`
  (returns (ImagePath :type String))
  (return (`KismetStringLibrary.Concat_StrStr` (`KismetSystemLibrary.GetProjectSavedDirectory`) (`KismetStringLibrary.Concat_StrStr` "/save-images/" (`self.SaveGameName`) ".png"))))

(fn `Load Data`
  (returns (`Actor Items` :type "Array of /Game/MasterRpgFramework/MasterInventory/Variables/Items/ST_Item Structure") (`Avaliable Recipes` :type "Array of DataTableRowHandle Structure") (`Max Slots` :type Integer) (`Slots Taken` :type Integer) (`Max Bags Slots` :type Integer) (`Action Slots Items` :type "Array of /Game/MasterRpgFramework/MasterInventory/Variables/Items/ST_Item Structure") (BagSlotsItem :type "Array of /Game/MasterRpgFramework/MasterInventory/Saving/ST_BagsSlots Structure") (ChestActors :type "Array of /Game/MasterRpgFramework/MasterInventory/Saving/ST_SaveGameChests Structure") (`Cooldown Items` :type "Array of /Game/MasterRpgFramework/MasterInventory/Saving/ST_CooldownItems Structure") (VendorActors :type "Array of /Game/MasterRpgFramework/MasterInventory/Saving/ST_SaveGameVendorActors Structure") (`Player Currency` :type Integer) (`Actor Quests` :type "Array of /Game/MasterRpgFramework/MasterInventory/Variables/QuestSystem/ST_Quests Structure") (`Actor Tutorial and tips` :type "Array of /Game/MasterRpgFramework/MasterInventory/Variables/TutorialAndTipsSystem/ST_Tutorial Structure") (`Character Attributes` :type "Array of /Game/MasterRpgFramework/MasterInventory/Variables/AttributePoints/ST_AtrributePoint Structure") (`Talent Points` :type Integer) (`Talent Points Spent` :type Integer) (`Character Talents` :type "Array of /Game/MasterRpgFramework/MasterInventory/Variables/TalentSystem/ST_CharacterTalent Structure") (PlayerSavedInputs :type "Array of EnhancedActionKeyMapping Structure"))
  (return (`self.Actor Items`) (`self.Avaliable Recipes`) (`self.Max Slots`) (`self.Slots Taken`) (`self.Max Bags Slots`) (`self.Action Slots Items`) (`self.BagSlotsItem`) (`self.ChestActors`) (`self.Cooldown Items`) (`self.VendorActors`) (`self.Player Currency`) (`self.Actor Quests`) (`self.Actor Tutorial and tips`) (`self.Character Attributes`) (`self.Talent Points`) (`self.Talent Points Spent`) (`self.Character Talents`) (`self.PlayerSavedInputs`)))

(fn `SaveData`
  (params (ActorItems :type "Array of /Game/MasterRpgFramework/MasterInventory/Variables/Items/ST_Item Structure") (AvaliableRecipes :type "Array of DataTableRowHandle Structure") (MaxSlots :type Integer) (SlotsTaken :type Integer) (MaxBagsSlots :type Integer) (ActionSlots :type "Array of /Game/MasterRpgFramework/MasterInventory/Ui/InventorySlots/WBP_ActionSlot Object Reference") (BagSlots :type "Array of /Game/MasterRpgFramework/MasterInventory/Ui/InventorySlots/WBP_Bag_Slot Object Reference") (ChestsActors :type "Array of /Game/MasterRpgFramework/MasterInventory/Blueprints/Chest/BP_BaseChest Object Reference") (CooldownItems :type "Array of /Game/MasterRpgFramework/MasterInventory/Saving/ST_CooldownItems Structure") (VendorActors :type "Array of /Game/MasterRpgFramework/MasterInventory/Blueprints/Vendor/BP_BaseVendor Object Reference") (`Player Currency` :type Integer) (ActorQuests :type "Array of /Game/MasterRpgFramework/MasterInventory/Variables/QuestSystem/ST_Quests Structure") (`Tutorial and tips` :type "Array of /Game/MasterRpgFramework/MasterInventory/Variables/TutorialAndTipsSystem/ST_Tutorial Structure") (CharacterAttributes :type "Array of /Game/MasterRpgFramework/MasterInventory/Variables/AttributePoints/ST_AtrributePoint Structure") (TalentPoints :type Integer) (TalentPointsSpent :type Integer) (CharacterTalents :type "Array of /Game/MasterRpgFramework/MasterInventory/Variables/TalentSystem/ST_CharacterTalent Structure") (SaveGameName :type String) (MappedInputs :type "Array of EnhancedActionKeyMapping Structure"))
  (bind (_year _month _day _hour _minute _second) (`KismetMathLibrary.BreakDateTime` (`KismetMathLibrary.Now`)))
  (`KismetArrayLibrary.Array_Clear` (`self.Actor Items`))
  (set `self.Actor Items` ActorItems)
  (`KismetArrayLibrary.Array_Clear` (`self.Avaliable Recipes`))
  (set `self.Avaliable Recipes` AvaliableRecipes)
  (set `self.Max Slots` MaxSlots)
  (set `self.Slots Taken` SlotsTaken)
  (set `self.Max Bags Slots` MaxBagsSlots)
  (`KismetArrayLibrary.Array_Clear` (`self.Action Slots Items`))
  (for _array_element ActionSlots
    (`KismetArrayLibrary.Array_Add` (`self.Action Slots Items`) (`/Game/MasterRpgFramework/MasterInventory/Ui/InventorySlots/WBP_ActionSlot.item` _array_element)))
  (`KismetArrayLibrary.Array_Clear` (`self.BagSlotsItem`))
  (for (_array_element_2 _array_index) BagSlots
    (`KismetArrayLibrary.Array_Add` (`self.BagSlotsItem`) (make `/Game/MasterRpgFramework/MasterInventory/Saving/ST_BagsSlots` _array_index (`/Game/MasterRpgFramework/MasterInventory/Ui/InventorySlots/WBP_Bag_Slot.item` _array_element_2))))
  (`KismetArrayLibrary.Array_Clear` (`self.ChestActors`))
  (for _array_element_3 ChestsActors
    ;[1 1 1] Save the dynamic chests
    (`KismetArrayLibrary.Array_Add` (`self.ChestActors`) (make `/Game/MasterRpgFramework/MasterInventory/Saving/ST_SaveGameChests` (`Actor.GetTransform` _array_element_3) (`/Game/ThirdPerson/Blueprints/BPC_MasterInventory.ActorItems` (`/Game/MasterRpgFramework/MasterInventory/Blueprints/Chest/BP_BaseChest.BP_MasterInventory` _array_element_3)) (`/Game/MasterRpgFramework/MasterInventory/Blueprints/Chest/BP_BaseChest.ChestId` _array_element_3) (`GameplayStatics.GetObjectClass` _array_element_3))))
  (set `self.Cooldown Items` CooldownItems)
  ;[1 1 1] Save the vendor actors
  (`KismetArrayLibrary.Array_Clear` (`self.VendorActors`))
  (for _array_element_4 VendorActors
    (`KismetArrayLibrary.Array_Add` (`self.VendorActors`) (make `/Game/MasterRpgFramework/MasterInventory/Saving/ST_SaveGameVendorActors` (`Actor.GetTransform` _array_element_4) (`/Game/ThirdPerson/Blueprints/BPC_MasterInventory.ActorItems` (`/Game/MasterRpgFramework/MasterInventory/Blueprints/Vendor/BP_BaseVendor.BP_MasterInventory` _array_element_4)) (`/Game/MasterRpgFramework/MasterInventory/Blueprints/Vendor/BP_BaseVendor.VendorId` _array_element_4) (`GameplayStatics.GetObjectClass` _array_element_4))))
  ;[1 1 1] Save the player currency
  (set `self.Player Currency` `Player Currency`)
  ;[1 1 1] Save the actor quests
  (`KismetArrayLibrary.Array_Clear` (`self.Actor Quests`))
  (for _array_element_5 ActorQuests
    (bind _structout (setmembers `/Game/MasterRpgFramework/MasterInventory/Variables/QuestSystem/ST_Quests` :`StructRef` _array_element_5))
    (`KismetArrayLibrary.Array_Add` (`self.Actor Quests`) _structout))
  ;[1 1 1] Save the actor tips and tutorial
  (`KismetArrayLibrary.Array_Clear` (`self.Actor Tutorial and tips`))
  (for _array_element_6 `Tutorial and tips`
    (`KismetArrayLibrary.Array_Add` (`self.Actor Tutorial and tips`) _array_element_6))
  ;[1 1 1] Character Attributes
  (set `self.Character Attributes` CharacterAttributes)
  ;[1 1 1] Save the player talents
  (set `self.Talent Points` TalentPoints)
  (set `self.Talent Points Spent` TalentPointsSpent)
  (set `self.Character Talents` CharacterTalents)
  ;[1 1 1] Save game slot
  (set `self.SaveGameName` SaveGameName)
  (set `self.SaveTimeStamp` (`KismetStringLibrary.Concat_StrStr` (`KismetStringLibrary.Conv_IntToString` _hour) ":" (`KismetStringLibrary.Conv_IntToString` _minute) ":" (`KismetStringLibrary.Conv_IntToString` _second) " " (`KismetStringLibrary.Conv_IntToString` _day) "/" (`KismetStringLibrary.Conv_IntToString` _month) "/" (`KismetStringLibrary.Conv_IntToString` _year)))
  (set `self.PlayerSavedInputs` MappedInputs)
  (return))