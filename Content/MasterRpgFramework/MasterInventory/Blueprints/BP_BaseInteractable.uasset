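; Base replicated interactable actor for the inventory framework, with optional mesh physics and overridable hooks for range, interaction and destruction.
; On authority, trigger overlaps find the Character's inventory through a controller interface, add or remove this actor as an interactable, and multicast range events that log in debug mode.
; Destruction is multicast, either immediate or after a smooth pickup timeline that shrinks the actor toward the interacting pawn.
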(event `self.ReceiveBeginPlay`
  ;[0 0.1366 0.5365 1 60] Check if this item can simulate physics
  (set `self.OriginalActorTransform` (`self.GetTransform` self))
  (if (`self.usePhysics`)
    (`PrimitiveComponent.SetSimulatePhysics` (`self.ItemMesh`) true)
    (else
      (`PrimitiveComponent.SetSimulatePhysics` (`self.ItemMesh`) false))))

(event `self.InventoryTrigger.OnComponentBeginOverlap`
  (params (OverlappedComponent :type "PrimitiveComponent Object Reference") (OtherActor :type "Actor Object Reference") (OtherComp :type "PrimitiveComponent Object Reference") (OtherBodyIndex :type Integer) (bFromSweep :type Boolean) (SweepResult :type "HitResult Structure (by ref)"))
  ;[0.03028 1 0 1 60] When the actor enter the range
  (bind _inventory (`self.ReturnInventory` OtherActor))
  (`/Engine/EditorBlueprintResources/StandardMacros.IsValid` _inventory
    (:`Is Valid`
      (`/Engine/EditorBlueprintResources/ActorMacros.Switch Has Authority`
        (:`Authority`
          (`self.Actor In Range Server` _inventory)
          (if (`self.Can Interact`)
            (`/Game/MasterRpgFramework/MasterInventory/Component/BPC_MasterInventory.Add Interactable Inventory Items (server)` _inventory self)))))))

(event `self.InventoryTrigger.OnComponentEndOverlap`
  (params (OverlappedComponent :type "PrimitiveComponent Object Reference") (OtherActor :type "Actor Object Reference") (OtherComp :type "PrimitiveComponent Object Reference") (OtherBodyIndex :type Integer))
  ;[1 0 0.0366 1 60] When the actor leave range
  (bind _inventory (`self.ReturnInventory` OtherActor))
  (`/Engine/EditorBlueprintResources/StandardMacros.IsValid` _inventory
    (:`Is Valid`
      (`/Engine/EditorBlueprintResources/ActorMacros.Switch Has Authority`
        (:`Authority`
          (`self.Actor Out Of Range Server` _inventory)
          (if (`self.Can Interact`)
            (`/Game/MasterRpgFramework/MasterInventory/Component/BPC_MasterInventory.Remove Interactable Inventory Items (server)` _inventory self)))))))

(event `Destroy_server`
  (params (Controller :type "PlayerController Object Reference"))
  ;[0 0 0 1 60] When the Actor gets destroy
  (`self.Destroy_multicast` Controller))

(event `Actor In Range Server`
  (params (InventoryRef :type "/Game/MasterRpgFramework/MasterInventory/Component/BPC_MasterInventory Object Reference"))
  ;[0 1 0.09182 1 60] When the actor leave the range
  (`self.Actor In Range Multicast` InventoryRef))

(event `Actor Out Of Range Server`
  (params (InventoryRef :type "/Game/MasterRpgFramework/MasterInventory/Component/BPC_MasterInventory Object Reference"))
  ;[1 0 0.0466 1 60] When the actor leave the range
  (`self.Actor Out Of Range Multicast` InventoryRef))

(event `Destroy_multicast`
  (params (PlayerController :type "PlayerController Object Reference"))
  ;[0 0 0 1 60] When the Actor gets destroy
  (if (`self.UseSmoothInteraction`)
    (`/Engine/EditorBlueprintResources/StandardMacros.IsValid` PlayerController
      (:`Is Valid`
        (`self.API_IntractionFx` (`Controller.K2_GetPawn` PlayerController)))
      (:`Is Not Valid`
        (`self.OnActorDestroy` :!label _label)))
    (else
      (goto _label))))

(event `Actor In Range Multicast`
  (params (InventoryRef :type "/Game/MasterRpgFramework/MasterInventory/Component/BPC_MasterInventory Object Reference"))
  ;[0 1 0.09182 1 60] When the actor leave the range
  (`self.ActorInRange` InventoryRef))

(event `Actor Out Of Range Multicast`
  (params (InventoryRef :type "/Game/MasterRpgFramework/MasterInventory/Component/BPC_MasterInventory Object Reference"))
  ;[1 0 0.0466 1 60] When the actor leave the range
  (`self.ActorOutOfRange` InventoryRef))

(event `API_InteractionCallBack_client`
  (params (GameController :type "PlayerController Object Reference") (InventoryReference :type "/Game/MasterRpgFramework/MasterInventory/Component/BPC_MasterInventory Object Reference"))
  ;[1 0.8219 0 1 60] When a actor interact with this actor we can trigger custom logic for each type
  (`self.Object Interaction Client` GameController InventoryReference))

(event `API_IntractionFx`
  (params (MoveToActorLocation :type "Actor Object Reference"))
  ;[1 1 1] This is a nice fx for when you want to pick items with the player
  (`PrimitiveComponent.SetSimulatePhysics` (`self.ItemMesh`) false)
  (set `self.CurrentActorScale` (`self.GetTransform`))
  (`PrimitiveComponent.SetCollisionEnabled` (`self.ItemMesh`) "NoCollision")
  (bind (_direction _newtrack_0) (`Timeline|SmoothPickup` :!via `PlayFromStart`)
    (:`Update`
      (`self.K2_SetActorTransform` (`KismetMathLibrary.TLerp` (`self.CurrentActorScale`) (`KismetMathLibrary.MakeTransform` (`self.K2_GetActorLocation` MoveToActorLocation) (.rotation (`self.CurrentActorScale`)) (0.01 0.01 0.01)) _newtrack_0)))
    (:`Finished`
      (`self.K2_DestroyActor`))))

(fn `ActorInRange`
  (params (InventoryRef :type "/Game/MasterRpgFramework/MasterInventory/Component/BPC_MasterInventory Object Reference"))
  (bind _maininventorywidget (`/Game/MasterRpgFramework/MasterInventory/Component/BPC_MasterInventory.MainInventoryWidget` InventoryRef))
  (`/Engine/EditorBlueprintResources/StandardMacros.IsValid` InventoryRef
    (:`Is Valid`
      ;[1 1 1] Debug mode?
      (if (`/Game/MasterRpgFramework/MasterInventory/Component/BPC_MasterInventory.In Debug` InventoryRef)
        (`/Game/MasterRpgFramework/MasterInventory/Ui/WBP_MainInventory.API_DisplayLogMessage` _maininventorywidget (`KismetTextLibrary.Conv_StringToText` (`KismetStringLibrary.Concat_StrStr` (`/Game/MasterRpgFramework/MasterInventory/Global/BFL_MasterHelperFunctions.Rich Text Tags to String` "text-green" (`KismetSystemLibrary.GetDisplayName` (`ActorComponent.GetOwner` InventoryRef))) " range of: " (`/Game/MasterRpgFramework/MasterInventory/Global/BFL_MasterHelperFunctions.Rich Text Tags to String` "text-yellow" (`KismetSystemLibrary.GetDisplayName` self)))) (`.debug_25_A630247C4523CF7B5B08F8B54818F274` (break `/Game/MasterRpgFramework/MasterUI/Widgets/Variables/ST_Icons` (`.icons_231_59DC80DA4E644FA7A47EB09620AAF252` (break `/Game/MasterRpgFramework/MasterUI/Widgets/ST_MasterUiSettings` (`/Game/MasterRpgFramework/MasterUI/Widgets/WBP_MasterUiBase.MasterUiSettings` _maininventorywidget))))) 0.0 "NewEnumerator5")
        (return)
        (else
          (return))))
    (:`Is Not Valid`
      (return))))

(fn `ActorOutOfRange`
  (params (InventoryRef :type "/Game/MasterRpgFramework/MasterInventory/Component/BPC_MasterInventory Object Reference"))
  (bind _maininventorywidget (`/Game/MasterRpgFramework/MasterInventory/Component/BPC_MasterInventory.MainInventoryWidget` InventoryRef))
  ;[1 1 1] Debug mode?
  (if (`/Game/MasterRpgFramework/MasterInventory/Component/BPC_MasterInventory.In Debug` InventoryRef)
    (`/Game/MasterRpgFramework/MasterInventory/Ui/WBP_MainInventory.API_DisplayLogMessage` _maininventorywidget (`KismetTextLibrary.Conv_StringToText` (`KismetStringLibrary.Concat_StrStr` (`/Game/MasterRpgFramework/MasterInventory/Global/BFL_MasterHelperFunctions.Rich Text Tags to String` "text-blue" (`KismetSystemLibrary.GetDisplayName` (`ActorComponent.GetOwner` InventoryRef))) " left range:" (`/Game/MasterRpgFramework/MasterInventory/Global/BFL_MasterHelperFunctions.Rich Text Tags to String` "text-red" (`KismetSystemLibrary.GetDisplayName` self)))) (`.debug_25_A630247C4523CF7B5B08F8B54818F274` (break `/Game/MasterRpgFramework/MasterUI/Widgets/Variables/ST_Icons` (`.icons_231_59DC80DA4E644FA7A47EB09620AAF252` (break `/Game/MasterRpgFramework/MasterUI/Widgets/ST_MasterUiSettings` (`/Game/MasterRpgFramework/MasterUI/Widgets/WBP_MasterUiBase.MasterUiSettings` _maininventorywidget))))) 0.0 "NewEnumerator5")
    (return)
    (else
      (return))))

(fn `Object Interaction Client`
  (params (PlayerControllerReference :type "PlayerController Object Reference") (InventoryReference :type "/Game/MasterRpgFramework/MasterInventory/Component/BPC_MasterInventory Object Reference"))
  (`KismetSystemLibrary.PrintString` "Pre actor interaction"))

(fn `OnActorDestroy`
  (`self.K2_DestroyActor`))

(fn `UserConstructionScript`)