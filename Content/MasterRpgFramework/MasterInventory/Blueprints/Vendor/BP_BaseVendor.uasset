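; Base vendor actor for the master inventory system, letting players open a vendor UI on an item stock held in its inventory component.
; On BeginPlay it optionally randomises its ID for dynamic spawning, then resolves starting items by row name and adds them with quantities.
; Interaction toggles the UI, locking out other users with a message unless simultaneous use is allowed.
; The current user going out of range releases the lock and closes the UI.
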(event `self.ReceiveBeginPlay`
  (`parent.ReceiveBeginPlay`)
  ;[1 1 1] If dynamic means that can be spawn at any time
  (if (`self.DynamicVendorId`)
    (set `self.VendorId` (`KismetMathLibrary.RandomIntegerInRange` 1000 9000)))
  (for _array_element (`self.VendorStartItems`)
    (bind (_item _qty) (break `/Game/MasterRpgFramework/MasterInventory/Variables/VendorSystem/ST_VendorStartItems` _array_element))
    (bind (_out_row _found) (`/Game/MasterRpgFramework/MasterInventory/Global/BFL_MasterHelperFunctions.Get Inventory Item` (`.RowName` (break `DataTableRowHandle` _item))))
    (if _found
      (bind _structout (setmembers `/Game/MasterRpgFramework/MasterInventory/Variables/Items/ST_Item` :`StructRef` _out_row :`Stack` _qty))
      (`/Game/MasterRpgFramework/MasterInventory/Component/BPC_MasterInventory.API_AddItem_server` (`self.BP_MasterInventory`) _structout false false false))))

(fn `ActorOutOfRange`
  (params (InventoryRef :type "/Game/MasterRpgFramework/MasterInventory/Component/BPC_MasterInventory Object Reference"))
  (bind _bp_masterinventory (`self.BP_MasterInventory`))
  (if (== InventoryRef (`self.UserReference`))
    (set `self.InUse` false)
    (`/Engine/EditorBlueprintResources/StandardMacros.IsValid` (`/Game/MasterRpgFramework/MasterInventory/Component/BPC_MasterInventory.VendorUIRef` _bp_masterinventory)
      (:`Is Valid`
        (`/Game/MasterRpgFramework/MasterInventory/Component/BPC_MasterInventory.CloseVendorUI` _bp_masterinventory InventoryRef)))))

(fn `Object Interaction Client`
  (params (PlayerControllerReference :type "PlayerController Object Reference") (InventoryReference :type "/Game/MasterRpgFramework/MasterInventory/Component/BPC_MasterInventory Object Reference"))
  (bind _bp_masterinventory (`self.BP_MasterInventory`))
  ;[1 0.1456 0] Is the chest in use
  (if (`self.InUse`)
    ;[1 0.8642 0] Is the same user ?
    (if (== InventoryReference (`self.UserReference`))
      ;[1 0.06447 0.6533] Logic the chest inventory WIDGET
      (set `/Game/MasterRpgFramework/MasterInventory/Component/BPC_MasterInventory.GameControler` PlayerControllerReference (`self.BP_MasterInventory`) :!label _label)
      (set `self.UserReference` InventoryReference)
      (`/Game/MasterRpgFramework/MasterInventory/Component/BPC_MasterInventory.ToogleVendor` _bp_masterinventory InventoryReference)
      (if (not (`self.simultaneous use`))
        (set `self.InUse` (`/Game/MasterRpgFramework/MasterInventory/Component/BPC_MasterInventory.isVendorOpen` _bp_masterinventory)))
      (else
        ;[1 1 1] Chest is currenlt in use
        (`/Game/MasterRpgFramework/MasterInventory/Component/BPC_MasterInventory.API_DisplayCustomMessage` (`local.InventoryReference`) "Vendor currently in use" null 5.0)))
    (else
      (goto _label))))

(fn `UserConstructionScript`
  (`parent.UserConstructionScript`))