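; Base path tracker actor that shows a navigation path to a destination actor with a Niagara effect.
; Each tick it recomputes the navmesh path from its sphere to PathDestination and feeds the points, endpoints pinned, into the effect's TargetPath array.
; A one-time line trace moves the sphere toward the floor once the referenced character is not falling.
; The actor destroys itself when the destination becomes invalid.
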(event `API_FindFloor`
  (bind _sphere (`self.Sphere`))
  (bind _returnvalue (`SceneComponent.K2_GetComponentLocation` (`self.Sphere`)))
  ;[1 1 1] On start we set this actor close to the floor as possible
  (bind (_outhit _returnvalue_2) (`KismetSystemLibrary.LineTraceSingle` _returnvalue (+ _returnvalue (`KismetMathLibrary.MakeVector` 0.0 0.0 (`self.Lince Trace Offset`))) "TraceTypeQuery1"))
  (if _returnvalue_2
    (`SceneComponent.K2_SetRelativeLocation` _sphere (- (`.Location` (`GameplayStatics.BreakHitResult` _outhit)) (`SceneComponent.K2_GetComponentLocation` _sphere)) false false)))

(event `self.ReceiveTick`
  (params (DeltaSeconds :type "Float (single-precision)"))
  (`/Engine/EditorBlueprintResources/StandardMacros.IsValid` (`self.PathDestination`)
    (:`Is Valid`
      (`self.API_StartReloadPathTracker`)
      ;[1 1 1] If the character is not falling we set the actor near the floor
      (if (not (`NavMovementComponent.IsFalling` (`Character.CharacterMovement` (`self.CharacterPawnRef`))))
        (`/Engine/EditorBlueprintResources/StandardMacros.DoOnce` false
          (:`Completed`
            (`self.API_FindFloor`)))))
    (:`Is Not Valid`
      (`self.K2_DestroyActor`))))

(event `API_StartReloadPathTracker`
  (`self.SetActorTickEnabled` true)
  (`/Engine/EditorBlueprintResources/StandardMacros.IsValid` (`self.NS_Path`)
    (:`Is Valid`
      _)
    (:`Is Not Valid`
      (bind _returnvalue (`NiagaraFunctionLibrary.SpawnSystemAttached` "/Game/MasterRpgFramework/MasterInventory/Blueprints/PathTracker/Vfx/NS_TargetPath.NS_TargetPath" (`self.Sphere`) "None" (0.0 0.0 0.0) (struct) "KeepRelativeOffset"))
      (set `self.NS_Path` _returnvalue)))
  ;[1 1 1] Fin the shorted path from the actor to the target
  (bind _returnvalue_2 (`NavigationSystemV1.FindPathToLocationSynchronously` (`SceneComponent.K2_GetComponentLocation` (`self.Sphere`)) (`self.K2_GetActorLocation` (`self.PathDestination`)) null null))
  (bind _pathpoints (`NavigationPath.PathPoints` _returnvalue_2))
  ;[1 1 1] Do we have a valid path ?
  (if (> (`KismetArrayLibrary.Array_LastIndex` _pathpoints) 0)
    (bind _output_get (set `self.Path Points` _pathpoints))
    ;[1 1 1] Get the path start
    (`KismetArrayLibrary.Array_Set` _output_get 0 (`SceneComponent.K2_GetComponentLocation` (`self.Sphere`)))
    ;[1 1 1] Get the last path
    (`KismetArrayLibrary.Array_Set` _output_get (`KismetArrayLibrary.Array_LastIndex` _output_get) (`self.K2_GetActorLocation` (`self.PathDestination`)))
    ;[1 1 1] Fill the gaps
    (`NiagaraDataInterfaceArrayFunctionLibrary.SetNiagaraArrayVector` (`self.NS_Path`) "TargetPath" _output_get)))

(fn `UserConstructionScript`)