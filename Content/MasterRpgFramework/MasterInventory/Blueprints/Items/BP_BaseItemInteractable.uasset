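; Base Blueprint for interactable inventory items that can show a world widget with item details when an actor comes into range.
; It extends the parent's in-range and out-of-range handlers to toggle that widget's visibility when the interaction-widget option is enabled.
; On entering range, it looks up the item and rarity rows, prints the rarity name, and sets the widget's name-and-quantity text in the rarity color.
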(fn `ActorInRange`
  (params (InventoryRef :type "/Game/ThirdPerson/Blueprints/BPC_MasterInventory Object Reference"))
  (`parent.ActorInRange` InventoryRef)
  (if (`self.UseInteractionWIdget`)
    (`SceneComponent.SetVisibility` (`self.Widget`) true false)
    (bind (_out_row _found) (`/Game/MasterRpgFramework/MasterInventory/Global/BFL_MasterHelperFunctions.Get Inventory Item` (`.RowName` (break `DataTableRowHandle` (`self.Item`)))))
    (if _found
      (bind ((`Name_6_4EEFF9644F2282ADBD11CA89BB42F2A7` _name) (`Rarity_19_DBCBD3674AF5D173E22CC3B9137A4B6B` _rarity)) (break `/Game/MasterRpgFramework/MasterInventory/Variables/Items/ST_Item` _out_row))
      (bind (_found_2 _out_row_2) (`/Game/MasterRpgFramework/MasterInventory/Global/BFL_MasterHelperFunctions.Get Rarity Info` (`.RowName` (break `DataTableRowHandle` _rarity))))
      (bind (_name_2 _color) (break `/Game/MasterRpgFramework/MasterInventory/Variables/Rarity/ST_Rarity` _out_row_2))
      (`KismetSystemLibrary.PrintString` _name_2)
      (bind _aswbp_item_widget (cast `/Game/MasterRpgFramework/MasterInventory/Blueprints/Items/Widget/WBP_ItemWidget` (`WidgetComponent.GetWidget` (`self.Widget`))))
      (`/Game/MasterRpgFramework/MasterInventory/Blueprints/Items/Widget/WBP_ItemWidget.API_SetValue` _aswbp_item_widget true (`KismetTextLibrary.Conv_NameToText` (`KismetStringLibrary.Conv_StringToName` (`KismetSystemLibrary.MakeLiteralString` (`KismetStringLibrary.Concat_StrStr` (`KismetStringLibrary.Conv_NameToString` _name) " x" (`KismetStringLibrary.Conv_IntToString` (`self.Qty`)))))) _color))))

(fn `ActorOutOfRange`
  (params (InventoryRef :type "/Game/ThirdPerson/Blueprints/BPC_MasterInventory Object Reference"))
  (`parent.ActorOutOfRange` InventoryRef)
  (if (`self.UseInteractionWIdget`)
    (`SceneComponent.SetVisibility` (`self.Widget`) false false)))

(fn `UserConstructionScript`
  (`parent.UserConstructionScript`))