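; Base chest actor that opens its own master inventory UI for one player at a time.
; Client-side interaction toggles the UI for the current user, or shows an in-use message to anyone else.
; When that user leaves range, the chest frees itself and closes the UI.
; Open/close state syncs through the player's inventory API for server access, and dynamic chests get a random ID on BeginPlay.
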(event `self.ReceiveBeginPlay`
  (`parent.ReceiveBeginPlay`)
  ;[1 1 1] If dynamic means that can be spawn at any time
  (if (`self.DynamicChestId`)
    (set `self.ChestId` (`KismetMathLibrary.RandomIntegerInRange` 1000 9000))))

(fn `ActorOutOfRange`
  (params (InventoryRef :type "/Game/ThirdPerson/Blueprints/BPC_MasterInventory Object Reference"))
  (bind _bp_masterinventory (`self.BP_MasterInventory`))
  (if (== InventoryRef (`self.UserReference`))
    (set `self.InUse` false)
    (`/Engine/EditorBlueprintResources/StandardMacros.IsValid` (`/Game/ThirdPerson/Blueprints/BPC_MasterInventory.MainInventoryWidget` _bp_masterinventory)
      (:`Is Valid`
        (`/Game/ThirdPerson/Blueprints/BPC_MasterInventory.CloseMainInventory` _bp_masterinventory)
        (bind _inventory (message `/Game/MasterRpgFramework/MasterInventory/Component/BPI_ActorInventory.I_ReturnInventoryReference` (`self.PlayerController`)))
        ;[1 1 1] Need to run on the server because we don;t have acess from this function
        (`/Game/ThirdPerson/Blueprints/BPC_MasterInventory.API_SyncChestOpenClose_client` _inventory self false)))))

(fn `Object Interaction Client`
  (params (PlayerControllerReference :type "PlayerController Object Reference") (InventoryReference :type "/Game/ThirdPerson/Blueprints/BPC_MasterInventory Object Reference"))
  (locals (PlayerControllerRef :type "PlayerController Object Reference") (`Inventory Ref` :type "/Game/ThirdPerson/Blueprints/BPC_MasterInventory Object Reference"))
  (set `local.PlayerControllerRef` PlayerControllerReference)
  (set `local.Inventory Ref` InventoryReference)
  ;[1 0.1456 0] Is the chest in use
  (if (`self.InUse`)
    ;[1 0.8642 0] Is the same user ?
    (if (== (`local.Inventory Ref`) (`self.UserReference`))
      ;[1 0.06447 0.6533] Logic the chest inventory WIDGET
      (bind _output_get (set `/Game/ThirdPerson/Blueprints/BPC_MasterInventory.GameControler` (`local.PlayerControllerRef`) (`self.BP_MasterInventory`) :!label _label))
      (set `self.PlayerController` _output_get)
      (if (`/Game/ThirdPerson/Blueprints/BPC_MasterInventory.Main Inventory Open` (`self.BP_MasterInventory`))
        ;[1 0.1379 0] Close the inventory ui
        (`/Game/ThirdPerson/Blueprints/BPC_MasterInventory.ToogleMainInventory` (`self.BP_MasterInventory`))
        (else
          ;[0.3916 1 0] Open the inventory ui
          (`/Game/ThirdPerson/Blueprints/BPC_MasterInventory.Start Main Inventory Widget` (`self.BP_MasterInventory`) _output_get)
          (`/Game/ThirdPerson/Blueprints/BPC_MasterInventory.ToogleMainInventory` (`self.BP_MasterInventory`))))
      (bind _output_get_2 (set `self.InUse` (`/Game/ThirdPerson/Blueprints/BPC_MasterInventory.Main Inventory Open` (`self.BP_MasterInventory`))))
      (set `self.UserReference` (`local.Inventory Ref`))
      ;[1 1 1] Need to run on the server because we don;t have acess from this function
      (`/Game/ThirdPerson/Blueprints/BPC_MasterInventory.API_SyncChestOpenClose_client` (`local.InventoryReference`) self _output_get_2)
      (else
        ;[1 1 1] Chest is currenlt in use
        (`/Game/ThirdPerson/Blueprints/BPC_MasterInventory.API_DisplayCustomMessage` (`local.InventoryReference`) "Chest currently in use" null 5.0)))
    (else
      (goto _label))))

(fn `UserConstructionScript`
  (`parent.UserConstructionScript`))