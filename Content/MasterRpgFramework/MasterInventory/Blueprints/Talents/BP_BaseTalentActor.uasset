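; Base actor for talents in the RPG inventory framework, providing hooks for when a character unlocks or reverts a talent.
; Server API events forward to multicast events, which call the UnlockTalent and TalentRevert functions.
; Both functions only print placeholder text, marking where talent-specific logic belongs.
; The actor is short-lived, destroying itself once DestroyTimer elapses after BeginPlay.
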(event `self.ReceiveBeginPlay`
  (`KismetSystemLibrary.Delay` (`self.DestroyTimer`))
  (`self.K2_DestroyActor`))

(event `API_UnlockTalent_server`
  ;[1 1 1] When the character unlock the talent
  (`self.API_UnlockTalent_Multicast`))

(event `API_UnlockTalent_Multicast`
  ;[1 1 1] When the character unlock the talent
  (`self.UnlockTalent`))

(event `API_TalentRevert_server`
  ;[1 1 1] When the player revert the talent
  (`self.API_TalentRevert_Multicast`))

(event `API_TalentRevert_Multicast`
  ;[1 1 1] When the player revert the talent
  (`self.TalentRevert`))

(fn `TalentRevert`
  (`KismetSystemLibrary.PrintString` "Talent revert logic"))

(fn `UnlockTalent`
  (`KismetSystemLibrary.PrintString` "You logic here"))

(fn `UserConstructionScript`)