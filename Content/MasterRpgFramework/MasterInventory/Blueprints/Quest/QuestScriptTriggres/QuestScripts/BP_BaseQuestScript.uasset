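; Base quest script actor that reacts to quest status changes and drives map guidance for that quest.
; The status API caches quest, status and inventory references, then calls HandleQuestEventStatus, which here only prints a debug message.
; Guidance APIs spawn markers through the inventory component, tagged with the quest ID.
; Removal passes through multicast and client events, destroys map markers matching an ID, then refreshes radar and map.
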(event `API_ScriptHandleQuestStatus`
  (params (QuestReference :type "/Game/MasterRpgFramework/MasterInventory/Variables/QuestSystem/ST_Quests Structure") (Status :type "/Game/MasterRpgFramework/MasterInventory/Variables/QuestSystem/E_QuestStatus Enum" :default "NewEnumerator0") (InventoryReference :type "/Game/ThirdPerson/Blueprints/BPC_MasterInventory Object Reference"))
  ;[1 0.06923 0.9924 1 60] Handle the quest script based in the quest status
  (set `self.QuestReference` QuestReference)
  (set `self.QuesStatusReference` Status)
  (set `self.Inventory Reference` InventoryReference)
  (`self.ScriptHandleQuestStatus` QuestReference Status InventoryReference))

(event `ScriptHandleQuestStatus`
  (params (Quest :type "/Game/MasterRpgFramework/MasterInventory/Variables/QuestSystem/ST_Quests Structure") (QuestStatus :type "/Game/MasterRpgFramework/MasterInventory/Variables/QuestSystem/E_QuestStatus Enum" :default "NewEnumerator0") (`Inventory Reference` :type "/Game/ThirdPerson/Blueprints/BPC_MasterInventory Object Reference"))
  ;[1 0.06923 0.9924 1 60] Handle the quest script based in the quest status
  (`self.HandleQuestEventStatus` Quest QuestStatus `Inventory Reference`))

(event `API_RemoveQuestMarkers`
  (params (MarkerId :type String))
  ;[0 0.7686 1 1 60] QUEST GUIDANCE SYSTEM
  ;;[1 0.1448 0.08836 1 60] Remove markers based in a given id
  (`self.RemoveQuestMarkers_multicast` MarkerId))

(event `RemoveQuestMarkers_multicast`
  (params (MarkerId :type String))
  ;[0 0.7686 1 1 60] QUEST GUIDANCE SYSTEM
  ;;[1 0.1448 0.08836 1 60] Remove markers based in a given id
  (`self.RemoveQuestMarkers_client` MarkerId))

(event `RemoveQuestMarkers_client`
  (params (MarkerId :type String))
  ;[0 0.7686 1 1 60] QUEST GUIDANCE SYSTEM
  ;;[1 0.1448 0.08836 1 60] Remove markers based in a given id
  (bind _outactors (`GameplayStatics.GetAllActorsOfClass` "/Game/MasterRpgFramework/MasterGuidanceSystem/Blueprints/MapMakers/BP_BaseMapMarker.BP_BaseMapMarker_C"))
  (for _array_element _outactors
    (if (`KismetStringLibrary.EqualEqual_StrStr` (`/Game/MasterRpgFramework/MasterGuidanceSystem/Blueprints/MapMakers/BP_BaseMapMarker.Marker Id` _array_element) MarkerId)
      (`self.K2_DestroyActor` _array_element)))
  (`self.API_RefreshRadarAndMap`))

(event `API_RefreshRadarAndMap`
  ;[0 0.7686 1 1 60] QUEST GUIDANCE SYSTEM
  ;;[1 0.7727 0 1 60] Force the refresh
  (`self.ForceRadarRefreshClient`))

(event `API_AddMarkers`
  (params (SpawnTransform :type "Transform Structure") (bCanBeRemoved :type Boolean) (bIsPlayerMarker :type Boolean) (bCanBeDiscover :type Boolean) (`Map MarkerTexture` :type "Texture2D Object Reference") (bDestoryOnTouch :type Boolean) (MarkerLegendName :type Text) (bSpawnPathTracker :type Boolean))
  ;[0 0.7686 1 1 60] QUEST GUIDANCE SYSTEM
  ;;[0 1 0.1618 1 60] Spawn the mark telling the player where to go on the client
  (`self.SpawnMarkerMulticastClient` SpawnTransform bCanBeRemoved bIsPlayerMarker bCanBeDiscover `Map MarkerTexture` bDestoryOnTouch MarkerLegendName bSpawnPathTracker))

(event `ForceRadarRefreshClient`
  ;[0 0.7686 1 1 60] QUEST GUIDANCE SYSTEM
  ;;[1 0.7727 0 1 60] Force the refresh
  (`/Game/ThirdPerson/Blueprints/BPC_MasterInventory.API_ForceGuidanceSystemRefresh` (`self.Inventory Reference`)))

(event `SpawnMarkerMulticastClient`
  (params (SpawnTransform :type "Transform Structure") (bCanBeRemoved :type Boolean) (bIsPlayerMarker :type Boolean) (bCanBeDiscover :type Boolean) (`Map MarkerTexture` :type "Texture2D Object Reference") (bDestoryOnTouch :type Boolean) (MarkerLegendName :type Text) (SpawnPathTracker :type Boolean))
  ;[0 0.7686 1 1 60] QUEST GUIDANCE SYSTEM
  ;;[0 1 0.1618 1 60] Spawn the mark telling the player where to go on the client
  (`/Game/ThirdPerson/Blueprints/BPC_MasterInventory.API_SpawnGuidanceMarker` (`self.Inventory Reference`) SpawnTransform bCanBeRemoved bIsPlayerMarker bCanBeDiscover `Map MarkerTexture` bDestoryOnTouch MarkerLegendName (`.ID_44_5F4C26A14C2826E2558A76BEFF83B2B3` (break `/Game/MasterRpgFramework/MasterInventory/Variables/QuestSystem/ST_Quests` (`self.QuestReference`))) SpawnPathTracker))

(fn `HandleQuestEventStatus`
  (params (Quest :type "/Game/MasterRpgFramework/MasterInventory/Variables/QuestSystem/ST_Quests Structure") (QuestStatus :type "/Game/MasterRpgFramework/MasterInventory/Variables/QuestSystem/E_QuestStatus Enum" :default "NewEnumerator0") (InventoryRef :type "/Game/ThirdPerson/Blueprints/BPC_MasterInventory Object Reference"))
  (bind ((`InventoryName_5_956821AB4D16D8B88CCB2E9306479F48` _inventoryname) (`DebugMode_30_F12FA0424EFC2B189B893C81FAD9F2C3` _debugmode)) (break `/Game/MasterRpgFramework/MasterInventory/Variables/InventorySettings/ST_InventorySettings` (`/Game/ThirdPerson/Blueprints/BPC_MasterInventory.Settings` InventoryRef)))
  (if _debugmode
    (`KismetSystemLibrary.PrintString` (`KismetStringLibrary.Concat_StrStr` (`KismetStringLibrary.Conv_NameToString` _inventoryname) " " "Has trigger the quest:" (`KismetStringLibrary.Conv_NameToString` (`.QuestName_6_45F694C0417B0C0852D8CBBFD37E42C2` (break `/Game/MasterRpgFramework/MasterInventory/Variables/QuestSystem/ST_Quests` Quest))) " " "Scripts") true true (struct :`R` 0.181814 :`G` 1.0 :`B` 0.261568 :`A` 1.0) 20.0))
  (return))

(fn `UserConstructionScript`)