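; Quest script for the demo quest "The Lost Sword", reacting to quest status changes through the parent's HandleQuestEventStatus.
; In Progress spawns a task-completion actor, sword pickup and map marker for the matching task ID, then plays a client-side cinematic with the UI hidden.
; Can Complete adds a return marker and appends another task to the quest.
; Completed or Abandon removes markers, spawned actors and the sword item from inventory.
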(event `SpawnTheSwordLocation`
  ;[0.07182 1 0.9569] Quest objects script activation
  ;;[1 0.2307 0.4356] Find the quest in the actor that trigger this action
  (bind (_valid _index _questinfo) (`/Game/ThirdPerson/Blueprints/BPC_MasterInventory.FindQuestOnActor` (`self.Inventory Reference`) (`self.QuestReference`)))
  (for _array_element (`.TasksProgress_37_3EE9FD7145A2B49AB8D35AA2C87A4003` (break `/Game/MasterRpgFramework/MasterInventory/Variables/QuestSystem/ST_Quests` _questinfo))
    ;;[0.2616 0.1711 1] Lets say you want to trigger special code for each task, all you need to know is the task id
    (set `self.QuestTask` _array_element)
    (switch `string` (`.ID_33_C62F127C45D3624876A08AA0A9F7551A` (break `/Game/MasterRpgFramework/MasterInventory/Variables/QuestSystem/QuestsTasks/ST_QuestTasks` _array_element))
      (:`#04`
        ;;[1 1 1] In here we are spawing the cubes based in the fisical locations base in the spawn points
        (bind _returnvalue (`|SpawnActorFromClass` "/Game/MasterRpgFramework/MasterInventory/Blueprints/Quest/QuestActors/BP_CompleteTaskBase.BP_CompleteTaskBase_C" (`KismetMathLibrary.Conv_VectorToTransform` (`KismetMathLibrary.TransformLocation` (`self.GetTransform`) (`self.SpawnSpointLocation`))) "Undefined" "OverrideRootScale" null (`self.Quest Target`) (`self.QuestTask`) true true false 1 "/Game/MasterRpgFramework/demo/UnrealAssets/LevelPrototyping/Materials/MI_Solid_Blue_Inst.MI_Solid_Blue_Inst" true 1 false true null))
        (bind _returnvalue_2 (`self.GetTransform` _returnvalue))
        (`self.API_AddMarkers` _returnvalue_2 false false true "/Game/MasterRpgFramework/MasterUI/Texture/Icons/GuidanceIcons/MainMarker.MainMarker" true "Marker" true)
        (bind _returnvalue_3 (`|SpawnActorFromClass` "/Game/MasterRpgFramework/MasterInventory/Blueprints/Items/ShowcaseItems/SworldExample/BP_SwordPicker.BP_SwordPicker_C" _returnvalue_2 "Undefined" "MultiplyWithRoot" null 1 false true null))
        (`KismetArrayLibrary.Array_Add` (`self.ActorsReference`) _returnvalue)
        (`KismetArrayLibrary.Array_Add` (`self.ActorsReference`) _returnvalue_3)
        (`KismetSystemLibrary.Delay` 2.0)
        ;;[1 1 1] Comes from the parent
        (`self.API_RefreshRadarAndMap`))))
  (`self.StartCinematic`))

(event `RemovePinkCubes`
  (bind _inventory_reference (`self.Inventory Reference`))
  ;[0.07182 1 0.9569] Quest objects script activation
  ;;[0.03646 0.03646 0.03646] case the player has cancel the quest we can destroy the actors, or do what you need
  (`self.API_RemoveQuestMarkers` (`.ID_44_5F4C26A14C2826E2558A76BEFF83B2B3` (break `/Game/MasterRpgFramework/MasterInventory/Variables/QuestSystem/ST_Quests` (`self.QuestReference`))))
  (for _array_element (`self.ActorsReference`)
    (`/Engine/EditorBlueprintResources/StandardMacros.IsValid` _array_element
      (:`Is Valid`
        (`self.K2_DestroyActor` _array_element))))
  (bind _out_row (`/Game/MasterRpgFramework/MasterInventory/Global/BFL_MasterHelperFunctions.Get Inventory Item` (`.RowName` (break `DataTableRowHandle` (`self.SwordItem`)))))
  (bind _item (`/Game/ThirdPerson/Blueprints/BPC_MasterInventory.Find Inventory Item` _inventory_reference _out_row false))
  (`/Game/ThirdPerson/Blueprints/BPC_MasterInventory.API_RemoveItem_server` _inventory_reference _item 1 true))

(event `SpawnReturnMarker`
  ;[0.07182 1 0.9569] Quest objects script activation
  ;;[1 1 1] Spawn the marker when the quest is redt to complete
  (`self.API_AddMarkers` (`KismetMathLibrary.Conv_VectorToTransform` (`KismetMathLibrary.TransformLocation` (`self.GetTransform`) (`self.FinalMarkerSpawn`))) false false true "/Game/MasterRpgFramework/MasterUI/Texture/Icons/GuidanceIcons/MainMarker.MainMarker" true "Main quest" true)
  (`KismetSystemLibrary.Delay` 1.0)
  (`self.API_RefreshRadarAndMap`)
  (bind (_found _out_row) (`/Game/MasterRpgFramework/MasterInventory/Global/BFL_MasterHelperFunctions.Get Quest Task` (`.RowName` (break `DataTableRowHandle` (`self.TaskToAppend`)))))
  (`/Game/ThirdPerson/Blueprints/BPC_MasterInventory.API_AppendTaskToQuest` (`self.Inventory Reference`) (`self.QuestReference`) _out_row))

(event `StartCinematic`
  ;[1 1 1] CINEMATIC ONLY RUN ON THE CLIENT :)
  (`self.StartCinematicCLient`))

(event `StartCinematicCLient`
  ;[1 1 1] CINEMATIC ONLY RUN ON THE CLIENT :)
  (`/Game/ThirdPerson/Blueprints/BPC_MasterInventory.API_ShowOrHideUi` (`self.Inventory Reference`) false)
  (bind _returnvalue (`|SpawnActorFromClass` "/Game/MasterRpgFramework/MasterCinematicManager/CInematicManager/BP_CinematicManager.BP_CinematicManager_C" (`KismetMathLibrary.MakeTransform` (0.0 0.0 0.0)) "Undefined" "MultiplyWithRoot" null "/Game/MasterRpgFramework/demo/CinematicDemo/TheLostSword/Sequence/TheLostSword.TheLostSword" true true true (`/Game/ThirdPerson/Blueprints/BPC_MasterInventory.GameControler` (`self.Inventory Reference`)) true true true "/Game/MasterRpgFramework/MasterCinematicManager/CinematicToPlayer/BP_NormalActorCamera.BP_NormalActorCamera_C" null))
  (add `/Game/MasterRpgFramework/MasterCinematicManager/CInematicManager/BP_CinematicManager.EV_CinematicComplete` _returnvalue (delegate `CinematicComplete`)))

(event `CinematicComplete`
  ;[1 1 1] CINEMATIC ONLY RUN ON THE CLIENT :)
  (`/Game/ThirdPerson/Blueprints/BPC_MasterInventory.API_ShowOrHideUi` (`self.Inventory Reference`) true))

(fn `HandleQuestEventStatus`
  (params (Quest :type "/Game/MasterRpgFramework/MasterInventory/Variables/QuestSystem/ST_Quests Structure") (QuestStatus :type "/Game/MasterRpgFramework/MasterInventory/Variables/QuestSystem/E_QuestStatus Enum" :default "NewEnumerator0") (InventoryRef :type "/Game/ThirdPerson/Blueprints/BPC_MasterInventory Object Reference"))
  (locals (QuestTargetStatus :type "/Game/MasterRpgFramework/MasterInventory/Variables/QuestSystem/E_QuestStatus Enum" :default "NewEnumerator0") (InventoryTrigger :type "/Game/ThirdPerson/Blueprints/BPC_MasterInventory Object Reference"))
  (set `self.Quest Target` Quest)
  (bind _output_get (set `local.QuestTargetStatus` QuestStatus))
  (bind _output_get_2 (set `local.InventoryTrigger` InventoryRef))
  (`parent.HandleQuestEventStatus` (`self.Quest Target`) _output_get _output_get_2)
  (switch `/Game/MasterRpgFramework/MasterInventory/Variables/QuestSystem/E_QuestStatus` (`local.QuestTargetStatus`)
    (:`NewEnumerator1`
      (`self.SpawnTheSwordLocation`))
    (:`NewEnumerator2`
      (`self.SpawnReturnMarker`))
    (:`NewEnumerator3`
      (`self.RemovePinkCubes` :!label _label))
    (:`NewEnumerator5`
      (goto _label))))

(fn `UserConstructionScript`
  (`parent.UserConstructionScript`))