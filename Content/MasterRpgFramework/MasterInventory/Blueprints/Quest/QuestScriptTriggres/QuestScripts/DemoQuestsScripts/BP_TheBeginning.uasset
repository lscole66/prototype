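; Demo quest script for "The Beginning" that reacts to quest status changes by managing task actors, map markers and an intro cinematic.
; In progress, it spawns task-completion cubes with markers at spawn points for the magic-items task, checking saved progress, and plays a client cinematic with the UI hidden.
; When completable, it adds a return marker and appends another task to the quest.
; On completion or abandonment, it removes markers and cubes.
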(event `SpawnMagicItems`
  ;[0.07182 1 0.9569] Quest objects script activation
  ;;[1 0.2307 0.4356] Find the quest in the actor that trigger this action
  (bind (_valid _index _questinfo) (`/Game/MasterRpgFramework/MasterInventory/Component/BPC_MasterInventory.FindQuestOnActor` (`self.Inventory Reference`) (`self.QuestReference`)))
  (for _array_element (`.TasksProgress_37_3EE9FD7145A2B49AB8D35AA2C87A4003` (break `/Game/MasterRpgFramework/MasterInventory/Variables/QuestSystem/ST_Quests` _questinfo))
    ;;[0.2616 0.1711 1] Lets say you want to trigger special code for each task, all you need to know is the task id
    (set `self.QuestTask` _array_element)
    (bind ((`ID_33_C62F127C45D3624876A08AA0A9F7551A` _id) (`RequiredItems_25_94DA8DBD42AF7AFF1A89199E943B051C` _requireditems)) (break `/Game/MasterRpgFramework/MasterInventory/Variables/QuestSystem/QuestsTasks/ST_QuestTasks` _array_element))
    (switch `string` _id
      (:`#3-magic-items`
        (set `self.TaskQty` (`.CurrentQty_8_822957584BC945493ABA97AF27513076` (break `/Game/MasterRpgFramework/MasterInventory/Variables/QuestSystem/QuestsTasks/ST_ItemRequiredType` _requireditems)))
        (for _array_element_2 (`self.CubesSpawnPoints`)
          ;;[0.5652 1 0.04407] This extra log is just a example where you a loding this quest from a save game and the player already has some complteded items in the task
          (set `self.CurrentLoop` (+ (`self.CurrentLoop`) 1))
          (if (== (`self.TaskQty`) 0)
            ;;[1 1 1] In here we are spawing the cubes based in the fisical locations base in the spawn points
            (bind _returnvalue (`|SpawnActorFromClass` "/Game/MasterRpgFramework/MasterInventory/Blueprints/Quest/QuestActors/BP_CompleteTaskBase.BP_CompleteTaskBase_C" (`KismetMathLibrary.Conv_VectorToTransform` (`KismetMathLibrary.TransformLocation` (`self.GetTransform`) _array_element_2)) "Undefined" "OverrideRootScale" null (`self.Quest Target`) (`self.QuestTask`) false true true 1 "/Game/MasterRpgFramework/demo/UnrealAssets/LevelPrototyping/Materials/MI_Solid_Blue.MI_Solid_Blue" true 1 false true null :!label _label))
            (`self.API_AddMarkers` (`self.GetTransform` _returnvalue) false false true "/Game/MasterRpgFramework/MasterUI/Texture/Icons/GuidanceIcons/SecondaryMarker.SecondaryMarker" true "Marker" true)
            (`KismetArrayLibrary.Array_Add` (`self.ActorsReference`) _returnvalue)
            (elif (<= (`self.CurrentLoop`) (`self.TaskQty`))
              (goto _label))))
        (`KismetSystemLibrary.Delay` 2.0)
        ;;[1 1 1] Comes from the parent
        (`self.API_RefreshRadarAndMap`))))
  (`self.StartCinematic`))

(event `StartCinematic`
  ;[0.07182 1 0.9569] Quest objects script activation
  ;;[1 1 1] CINEMATIC ONLY RUN ON THE CLIENT :)
  (`self.StartCinematicCLient`))

(event `StartCinematicCLient`
  ;[0.07182 1 0.9569] Quest objects script activation
  ;;[1 1 1] CINEMATIC ONLY RUN ON THE CLIENT :)
  (`/Game/MasterRpgFramework/MasterInventory/Component/BPC_MasterInventory.API_ShowOrHideUi` (`self.Inventory Reference`) false)
  (bind _returnvalue (`|SpawnActorFromClass` "/Game/MasterRpgFramework/MasterCinematicManager/CInematicManager/BP_CinematicManager.BP_CinematicManager_C" (`KismetMathLibrary.MakeTransform` (0.0 0.0 0.0)) "Undefined" "MultiplyWithRoot" null "/Game/MasterRpgFramework/demo/CinematicDemo/TheBeggining/TheBeggining/TheBegginingRoot.TheBegginingRoot" true true true (`/Game/MasterRpgFramework/MasterInventory/Component/BPC_MasterInventory.GameControler` (`self.Inventory Reference`)) true true true "/Game/MasterRpgFramework/MasterCinematicManager/CinematicToPlayer/BP_NormalActorCamera.BP_NormalActorCamera_C" null))
  (add `/Game/MasterRpgFramework/MasterCinematicManager/CInematicManager/BP_CinematicManager.EV_CinematicComplete` _returnvalue (delegate `CinematicComplete`)))

(event `CinematicComplete`
  ;[0.07182 1 0.9569] Quest objects script activation
  ;;[1 1 1] CINEMATIC ONLY RUN ON THE CLIENT :)
  (`/Game/MasterRpgFramework/MasterInventory/Component/BPC_MasterInventory.API_ShowOrHideUi` (`self.Inventory Reference`) true))

(event `RemovePinkCubes`
  ;[0.07182 1 0.9569] Quest objects script activation
  ;;[0.03646 0.03646 0.03646] case the player has cancel the quest we can destroy the actors, or do what you need
  (`self.API_RemoveQuestMarkers` (`.ID_44_5F4C26A14C2826E2558A76BEFF83B2B3` (break `/Game/MasterRpgFramework/MasterInventory/Variables/QuestSystem/ST_Quests` (`self.QuestReference`))))
  (for _array_element (`self.ActorsReference`)
    (`/Engine/EditorBlueprintResources/StandardMacros.IsValid` _array_element
      (:`Is Valid`
        (`self.K2_DestroyActor` _array_element)))))

(event `SpawnReturnMarker`
  ;[0.07182 1 0.9569] Quest objects script activation
  ;;[1 1 1] Spawn the marker when the quest is redt to complete
  (`self.API_AddMarkers` (`KismetMathLibrary.Conv_VectorToTransform` (`KismetMathLibrary.TransformLocation` (`self.GetTransform`) (`self.FinalMarkerSpawn`))) false false true "/Game/MasterRpgFramework/MasterUI/Texture/Icons/GuidanceIcons/SecondaryMarker.SecondaryMarker" true "Main quest" true)
  (`KismetSystemLibrary.Delay` 1.0)
  (`self.API_RefreshRadarAndMap`)
  (bind (_found _out_row) (`/Game/MasterRpgFramework/MasterInventory/Global/BFL_MasterHelperFunctions.Get Quest Task` (`.RowName` (break `DataTableRowHandle` (`self.TaskToAppend`)))))
  (`/Game/MasterRpgFramework/MasterInventory/Component/BPC_MasterInventory.API_AppendTaskToQuest` (`self.Inventory Reference`) (`self.QuestReference`) _out_row))

(fn `HandleQuestEventStatus`
  (params (Quest :type "/Game/MasterRpgFramework/MasterInventory/Variables/QuestSystem/ST_Quests Structure") (QuestStatus :type "/Game/MasterRpgFramework/MasterInventory/Variables/QuestSystem/E_QuestStatus Enum" :default "NewEnumerator0") (InventoryRef :type "/Game/MasterRpgFramework/MasterInventory/Component/BPC_MasterInventory Object Reference"))
  (locals (QuestTargetStatus :type "/Game/MasterRpgFramework/MasterInventory/Variables/QuestSystem/E_QuestStatus Enum" :default "NewEnumerator0") (InventoryTrigger :type "/Game/MasterRpgFramework/MasterInventory/Component/BPC_MasterInventory Object Reference"))
  (set `self.Quest Target` Quest)
  (bind _output_get (set `local.QuestTargetStatus` QuestStatus))
  (bind _output_get_2 (set `local.InventoryTrigger` InventoryRef))
  (`parent.HandleQuestEventStatus` (`self.Quest Target`) _output_get _output_get_2)
  (switch `/Game/MasterRpgFramework/MasterInventory/Variables/QuestSystem/E_QuestStatus` (`local.QuestTargetStatus`)
    (:`NewEnumerator1`
      (`self.SpawnMagicItems`))
    (:`NewEnumerator2`
      (`self.SpawnReturnMarker`))
    (:`NewEnumerator3`
      (`self.RemovePinkCubes` :!label _label))
    (:`NewEnumerator5`
      (goto _label))))

(fn `UserConstructionScript`
  (`parent.UserConstructionScript`))