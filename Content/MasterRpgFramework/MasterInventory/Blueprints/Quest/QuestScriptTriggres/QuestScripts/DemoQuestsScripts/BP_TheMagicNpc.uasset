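; Demo quest script actor for the magic NPC quest, reacting to quest status changes through an override of HandleQuestEventStatus.
; In progress, it places a map marker with path tracker and a task-completion actor at the NPC location for the matching task ID.
; When ready to complete, it adds a final marker and appends another task to the quest.
; Completion or abandonment removes quest markers and destroys spawned actors.
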(event `SpawnMagicItems`
  (bind _returnvalue (`KismetMathLibrary.Conv_VectorToTransform` (`KismetMathLibrary.TransformLocation` (`self.GetTransform`) (`self.NpcMarker`))))
  ;[0.07182 1 0.9569] Quest objects script activation
  ;;[1 0.2307 0.4356] Find the quest in the actor that trigger this action
  (bind (_valid _index _questinfo) (`/Game/ThirdPerson/Blueprints/BPC_MasterInventory.FindQuestOnActor` (`self.Inventory Reference`) (`self.QuestReference`)))
  (for _array_element (`.TasksProgress_37_3EE9FD7145A2B49AB8D35AA2C87A4003` (break `/Game/MasterRpgFramework/MasterInventory/Variables/QuestSystem/ST_Quests` _questinfo))
    ;;[0.2616 0.1711 1] Lets say you want to trigger special code for each task, all you need to know is the task id
    (set `self.QuestTask` _array_element)
    (switch `string` (`.ID_33_C62F127C45D3624876A08AA0A9F7551A` (break `/Game/MasterRpgFramework/MasterInventory/Variables/QuestSystem/QuestsTasks/ST_QuestTasks` _array_element))
      (:`#the-npc`
        (`self.API_AddMarkers` _returnvalue false false true "/Game/MasterRpgFramework/MasterUI/Texture/Icons/GuidanceIcons/SecondaryMarker.SecondaryMarker" true "Main quest" true)
        (bind _returnvalue_2 (`|SpawnActorFromClass` "/Game/MasterRpgFramework/MasterInventory/Blueprints/Quest/QuestActors/BP_CompleteTaskBase.BP_CompleteTaskBase_C" _returnvalue "Undefined" "OverrideRootScale" null (`self.Quest Target`) (`self.QuestTask`) false true true 1 "/Game/MasterRpgFramework/demo/UnrealAssets/LevelPrototyping/Materials/MI_Solid_Blue.MI_Solid_Blue" true 1 false true null))
        (`KismetArrayLibrary.Array_Add` (`self.ActorsReference`) _returnvalue_2))))
  (`KismetSystemLibrary.Delay` 1.0)
  (`self.API_RefreshRadarAndMap`))

(event `RemovePinkCubes`
  ;[0.07182 1 0.9569] Quest objects script activation
  ;;[0.03646 0.03646 0.03646] case the player has cancel the quest we can destroy the actors, or do what you need
  (`self.API_RemoveQuestMarkers` (`.ID_44_5F4C26A14C2826E2558A76BEFF83B2B3` (break `/Game/MasterRpgFramework/MasterInventory/Variables/QuestSystem/ST_Quests` (`self.QuestReference`))))
  (for _array_element (`self.ActorsReference`)
    (`/Engine/EditorBlueprintResources/StandardMacros.IsValid` _array_element
      (:`Is Valid`
        (`self.K2_DestroyActor` _array_element)))))

(event `SpawnReturnMarker`
  ;[0.07182 1 0.9569] Quest objects script activation
  ;;[1 1 1] Spawn the marker when the quest is redt to complete
  (`self.API_AddMarkers` (`KismetMathLibrary.Conv_VectorToTransform` (`KismetMathLibrary.TransformLocation` (`self.GetTransform`) (`self.FinalMarker`))) false false true "/Game/MasterRpgFramework/MasterUI/Texture/Icons/GuidanceIcons/SecondaryMarker.SecondaryMarker" true "Main quest" true)
  (`KismetSystemLibrary.Delay` 1.0)
  (`self.API_RefreshRadarAndMap`)
  (bind (_found _out_row) (`/Game/MasterRpgFramework/MasterInventory/Global/BFL_MasterHelperFunctions.Get Quest Task` (`.RowName` (break `DataTableRowHandle` (`self.TaskToAppend`)))))
  (`/Game/ThirdPerson/Blueprints/BPC_MasterInventory.API_AppendTaskToQuest` (`self.Inventory Reference`) (`self.QuestReference`) _out_row))

(fn `HandleQuestEventStatus`
  (params (Quest :type "/Game/MasterRpgFramework/MasterInventory/Variables/QuestSystem/ST_Quests Structure") (QuestStatus :type "/Game/MasterRpgFramework/MasterInventory/Variables/QuestSystem/E_QuestStatus Enum" :default "NewEnumerator0") (InventoryRef :type "/Game/ThirdPerson/Blueprints/BPC_MasterInventory Object Reference"))
  (locals (QuestTargetStatus :type "/Game/MasterRpgFramework/MasterInventory/Variables/QuestSystem/E_QuestStatus Enum" :default "NewEnumerator0") (InventoryTrigger :type "/Game/ThirdPerson/Blueprints/BPC_MasterInventory Object Reference"))
  (set `self.Quest Target` Quest)
  (bind _output_get (set `local.QuestTargetStatus` QuestStatus))
  (bind _output_get_2 (set `local.InventoryTrigger` InventoryRef))
  (`parent.HandleQuestEventStatus` (`self.Quest Target`) _output_get _output_get_2)
  (switch `/Game/MasterRpgFramework/MasterInventory/Variables/QuestSystem/E_QuestStatus` (`local.QuestTargetStatus`)
    (:`NewEnumerator1`
      (`self.SpawnMagicItems`))
    (:`NewEnumerator2`
      (`self.SpawnReturnMarker`))
    (:`NewEnumerator3`
      (`self.RemovePinkCubes` :!label _label))
    (:`NewEnumerator5`
      (goto _label))))

(fn `UserConstructionScript`
  (`parent.UserConstructionScript`))