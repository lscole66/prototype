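; BP_QuestWorldManager routes quest status changes to the script actors that run each quest's world logic.
; It matches the incoming quest's ID against its ManagedQuests list, resolving each entry's data table row, and forwards the status and inventory reference to that entry's script actor.
; If no valid actor exists, it spawns one from the entry's class at the manager's transform and stores the reference in the list for reuse.
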(event `API_TriggerHandleQuestStatus`
  (params (Quest :type "/Game/MasterRpgFramework/MasterInventory/Variables/QuestSystem/ST_Quests Structure") (QuestStatus :type "/Game/MasterRpgFramework/MasterInventory/Variables/QuestSystem/E_QuestStatus Enum" :default "NewEnumerator0") (InventoryReference :type "/Game/MasterRpgFramework/MasterInventory/Component/BPC_MasterInventory Object Reference"))
  ;[0.3137 0 1] THIS EVENT WILL FIND THE QUEST ON THE MANAGER IF THERE IS ONE TO BE FOUND AND TRIGGER THE EVENT TO START THE QUEST
  (`self.TriggerHandleQuestStatus` Quest QuestStatus InventoryReference))

(event `TriggerHandleQuestStatus`
  (params (Quest :type "/Game/MasterRpgFramework/MasterInventory/Variables/QuestSystem/ST_Quests Structure") (QuestStatus :type "/Game/MasterRpgFramework/MasterInventory/Variables/QuestSystem/E_QuestStatus Enum" :default "NewEnumerator0") (InventoryReference :type "/Game/MasterRpgFramework/MasterInventory/Component/BPC_MasterInventory Object Reference"))
  (bind ((`QuestScriptActor_5_707E32ED4AB874ABBA63FEA8422BEFEC` _questscriptactor) (`QuestScriptClass_8_E833093D4A3B349C10DC6A9D9BBB1A7B` _questscriptclass)) (break `/Game/MasterRpgFramework/MasterInventory/Blueprints/Quest/QuestScriptTriggres/WorldManager/ST_QuestManager` (`self.TempLoopManagerQuest`)))
  ;[0.3137 0 1] THIS EVENT WILL FIND THE QUEST ON THE MANAGER IF THERE IS ONE TO BE FOUND AND TRIGGER THE EVENT TO START THE QUEST
  (set `self.QuestTarget` Quest)
  (set `self.QuestStatusTarget` QuestStatus)
  (for (_array_element _array_index) (`self.ManagedQuests`)
    (set `self.TempLoopManagerQuest` _array_element)
    (set `self.MangeQuestIndex` _array_index)
    (bind (_found _out_row) (`/Game/MasterRpgFramework/MasterInventory/Global/BFL_MasterHelperFunctions.Get Quest Info` (`.RowName` (break `DataTableRowHandle` (`.Quest_3_0C1B52764143BC348B22209C7EB78996` (break `/Game/MasterRpgFramework/MasterInventory/Blueprints/Quest/QuestScriptTriggres/WorldManager/ST_QuestManager` _array_element))))))
    (if _found
      ;;[1 1 1] Check if the quest manager have the quest before we can trigger events
      (if (`KismetStringLibrary.EqualEqual_StrStr` (`.ID_44_5F4C26A14C2826E2558A76BEFF83B2B3` (break `/Game/MasterRpgFramework/MasterInventory/Variables/QuestSystem/ST_Quests` _out_row)) (`.ID_44_5F4C26A14C2826E2558A76BEFF83B2B3` (break `/Game/MasterRpgFramework/MasterInventory/Variables/QuestSystem/ST_Quests` (`self.QuestTarget`))))
        ;;[1 1 1] If the quest script actor valid ?
        (`/Engine/EditorBlueprintResources/StandardMacros.IsValid` _questscriptactor
          (:`Is Valid`
            (`/Game/MasterRpgFramework/MasterInventory/Blueprints/Quest/QuestScriptTriggres/QuestScripts/BP_BaseQuestScript.API_ScriptHandleQuestStatus` _questscriptactor (`self.QuestTarget`) (`self.QuestStatusTarget`) InventoryReference))
          (:`Is Not Valid`
            ;[1 0 0.07349] THIS PART WILL HANDLE IF WE HAVE A DYNAMIC SPAWN ACTOR, NOTE THAT IF YOU SPAWN THIS ACTOR IT WILL BE SET THE REFERENCE IN THE MANAGER QUEST SO WE DON;T NEED TO SPAWN THE SAME ACTOR TWICE
            (if (`KismetSystemLibrary.IsValidClass` _questscriptclass)
              (bind _returnvalue (`|SpawnActorFromClass` _questscriptclass (`self.GetTransform`) "Undefined" "SelectDefaultAtRuntime" null null))
              (`/Game/MasterRpgFramework/MasterInventory/Blueprints/Quest/QuestScriptTriggres/QuestScripts/BP_BaseQuestScript.API_ScriptHandleQuestStatus` _returnvalue (`self.QuestTarget`) (`self.QuestStatusTarget`) InventoryReference)
              (setmembers `/Game/MasterRpgFramework/MasterInventory/Blueprints/Quest/QuestScriptTriggres/WorldManager/ST_QuestManager` :`StructRef` (`|GetArrayItem` (`self.ManagedQuests`) (`self.MangeQuestIndex`)) :`QuestScriptActor` _returnvalue))))))))

(fn `UserConstructionScript`)