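; Base quest giver actor for the RPG framework that offers its configured quests through an inventory-driven window.
; On BeginPlay it optionally randomizes its ID for dynamic spawning, then looks up each available quest's row and registers it with its BPMasterInventory.
; Client interaction toggles the quest window, using an in-use lock to turn away other players unless simultaneous use is allowed.
; When the current user leaves range, it releases the lock and closes the window.
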(event `self.ReceiveBeginPlay`
  (`parent.ReceiveBeginPlay`)
  ;[1 0.3172 0 1 60] If dynamic means that can be spawn at any time
  (if (`self.DynamicQuestGiverId`)
    (set `self.QuestGiverID` (`KismetMathLibrary.RandomIntegerInRange` 9000 10000)))
  ;[0.7847 1 0.02455 1 60] Adds the quest to the actor component so we can see in the widget ui
  (for _array_element (`self.NpcAvailableQuests`)
    (bind (_quest_datatable _quest_rowname) (break `DataTableRowHandle` (break `/Game/MasterRpgFramework/MasterInventory/Blueprints/Quest/QuestGiver/ST_NpcAvailableQuests` _array_element)))
    (bind (_found _out_row) (`/Game/MasterRpgFramework/MasterInventory/Global/BFL_MasterHelperFunctions.Get Quest Info` _quest_rowname))
    (`/Game/MasterRpgFramework/MasterInventory/Component/BPC_MasterInventory.API_AddQuestGiver_server` (`self.BP_MasterInventory`) _out_row)))

(fn `ActorOutOfRange`
  (params (InventoryRef :type "/Game/MasterRpgFramework/MasterInventory/Component/BPC_MasterInventory Object Reference"))
  (if (== InventoryRef (`self.UserReference`))
    (set `self.InUse` false)
    (`/Engine/EditorBlueprintResources/StandardMacros.IsValid` (`/Game/MasterRpgFramework/MasterInventory/Component/BPC_MasterInventory.QuestGiverUiRef` (`self.BP_MasterInventory`))
      (:`Is Valid`
        (`/Game/MasterRpgFramework/MasterInventory/Component/BPC_MasterInventory.CloseQuestGiverWindow` (`self.BP_MasterInventory`) InventoryRef)))))

(fn `Object Interaction Client`
  (params (PlayerControllerReference :type "PlayerController Object Reference") (InventoryReference :type "/Game/MasterRpgFramework/MasterInventory/Component/BPC_MasterInventory Object Reference"))
  (bind _bp_masterinventory (`self.BP_MasterInventory`))
  ;[1 0.1456 0] Is the actor in use
  (if (`self.InUse`)
    ;[1 0.8642 0] Is the same user ?
    (if (== InventoryReference (`self.UserReference`))
      ;[1 0.06447 0.6533] Logic the quest giver inventory WIDGET
      (set `/Game/MasterRpgFramework/MasterInventory/Component/BPC_MasterInventory.GameControler` PlayerControllerReference (`self.BP_MasterInventory`) :!label _label)
      (bind _output_get (set `self.UserReference` InventoryReference))
      (`/Game/MasterRpgFramework/MasterInventory/Component/BPC_MasterInventory.ToogleQuestGiverWindow` _bp_masterinventory _output_get)
      (if (not (`self.simultaneous use`))
        (set `self.InUse` (`/Game/MasterRpgFramework/MasterInventory/Component/BPC_MasterInventory.isVendorOpen` _bp_masterinventory)))
      (else
        ;[1 1 1] Actor is currenlt in use
        (`/Game/MasterRpgFramework/MasterInventory/Component/BPC_MasterInventory.API_DisplayCustomMessage` (`local.InventoryReference`) "Npc currently in use" null 5.0)))
    (else
      (goto _label))))

(fn `UserConstructionScript`
  (`parent.UserConstructionScript`))