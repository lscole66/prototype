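; BP_CompleteTaskBase is a quest actor that advances a target quest task when an actor comes in range.
; ActorInRange runs on authority only and switches on the task type, calling the inventory API.
; Reach tasks set completion, while Action tasks add or remove required quantity, both passing a destroy-on-success option.
; The construction script optionally overrides the item mesh material.
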(fn `ActorInRange`
  (params (InventoryRef :type "/Game/MasterRpgFramework/MasterInventory/Component/BPC_MasterInventory Object Reference"))
  (`parent.ActorInRange` InventoryRef)
  (`/Engine/EditorBlueprintResources/ActorMacros.Switch Has Authority`
    (:`Authority`
      (switch `/Game/MasterRpgFramework/MasterInventory/Variables/QuestSystem/QuestsTasks/E_TaskTypes` (`.TaskType_27_215760C64B6ADA2B680DCC928681B77C` (break `/Game/MasterRpgFramework/MasterInventory/Variables/QuestSystem/QuestsTasks/ST_QuestTasks` (`self.QuestTaskTarget`)))
        (:`NewEnumerator2`
          ;[1 1 1 1 60] Reach destination task example
          (`/Game/MasterRpgFramework/MasterInventory/Component/BPC_MasterInventory.API_SetCompleteTask` InventoryRef (`self.QuestTarget`) (`self.QuestTaskTarget`) (`self.CompleteTask?`) (`self.DestroyOnSucess`) self))
        (:`NewEnumerator3`
          ;[1 1 1 1 60] Task based in actions example
          (`/Game/MasterRpgFramework/MasterInventory/Component/BPC_MasterInventory.API_SetTaskRequiredQty` InventoryRef (`self.QuestTarget`) (`self.QuestTaskTarget`) (`self.DestroyOnSucess`) self (`self.Is Adding`) (`self.AddingOrRemoveingActionQty`)))))))

(fn `UserConstructionScript`
  (`parent.UserConstructionScript`)
  (if (`self.DynamicChangeMaterial`)
    (`PrimitiveComponent.SetMaterial` (`self.ItemMesh`) 0 (`self.Material`))))