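; Base transition camera actor that hands the view from a cinematic back to the player's camera.
; API_StartTranstion disables the controlled pawn's input, makes itself the view target and runs a timeline that lerps its transform toward the live player camera.
; Each update blends from the actor's current transform, so the alpha compounds.
; On finish it returns view and input to the pawn, calls CallTransitionFinish, then destroys itself after a short delay.
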(event `API_StartTranstion`
  (params (PlayerController :type "PlayerController Object Reference") (PlayerCamera :type "CameraComponent Object Reference"))
  (bind _targetplayercontroller (`self.TargetPlayerController`))
  (bind _targetplayercontroller_2 (`self.TargetPlayerController`))
  (bind _targetplayercontroller_3 (`self.TargetPlayerController`))
  (set `self.TargetPlayerController` PlayerController)
  (set `self.PlayerCamera` PlayerCamera)
  (`self.DisableInput` (`Controller.K2_GetPawn` _targetplayercontroller) _targetplayercontroller)
  (`PlayerController.SetViewTargetWithBlend` (`self.TargetPlayerController`) self 0.0 "VTBlend_Linear" 0.0 false)
  (bind (_direction _transition) (`Timeline|Transition` :!via `PlayFromStart`)
    (:`Update`
      (`self.K2_SetActorTransform` self (`KismetMathLibrary.TLerp` (`self.GetTransform` self) (`SceneComponent.K2_GetComponentToWorld` (`self.PlayerCamera`)) _transition) false false))
    (:`Finished`
      (`PlayerController.SetViewTargetWithBlend` _targetplayercontroller_2 (`Controller.K2_GetPawn` _targetplayercontroller_2) 0.0 "VTBlend_Linear" 0.0 false)
      (`self.EnableInput` (`Controller.K2_GetPawn` _targetplayercontroller_3) _targetplayercontroller_3)
      (`self.TransitionFinish`)
      (`KismetSystemLibrary.Delay` 0.2)
      (`self.K2_DestroyActor`))))

(fn `UserConstructionScript`)