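; BP_CinematicManager is an actor that plays a level sequence, on BeginPlay or on demand, with a widget for pausing and skipping.
; It can disable pawn input during playback and broadcasts play, pause, stop and completion events.
; Tick caches the active cinematic camera transform.
; On finish or stop, it optionally spawns a camera actor there to blend back to the player camera, then completes and can destroy itself.
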(event `API_Boot`
  (params (PlayerController :type "PlayerController Object Reference"))
  ;[1 1 1] Set the player controller
  (set `self.PlayerController` PlayerController))

(event `self.ReceiveBeginPlay`
  ;[1 1 1] Auto play the cinematic
  (if (`self.AutoPlay`)
    (`self.API_PlayCinematic` 1.0)))

(event `API_PlayCinematic`
  (params (`Play Rate` :type "Float (single-precision)" :default 1.0))
  (bind _cinematiccontrollwidget (`self.CinematicControllWidget`))
  (bind _playercontroller (`self.PlayerController`))
  (`self.EV_CinematicPlay`)
  (bind _returnvalue (`|CreateWidget` "/Game/MasterRpgFramework/MasterCinematicManager/Widget/WBP_CinematicSkip.WBP_CinematicSkip_C" null self))
  (bind _output_get (set `self.CinematicControllWidget` _returnvalue))
  (add `/Game/MasterRpgFramework/MasterCinematicManager/Widget/WBP_CinematicSkip.Event_CinematicSkip` _cinematiccontrollwidget (delegate `CinematicStop`))
  (add `/Game/MasterRpgFramework/MasterCinematicManager/Widget/WBP_CinematicSkip.Event_CinematicPlayOrPause` _cinematiccontrollwidget (delegate `CinematicPause or Unpause`))
  (`UserWidget.AddToViewport` _output_get 0)
  (`/Engine/EditorBlueprintResources/StandardMacros.IsValid` (`self.PlayerController`)
    (:`Is Valid`
      ;[1 1 1] Do we want to disable the player input
      (if (`self.DisablePlayerInputs`)
        (`self.DisableInput` (`Controller.K2_GetPawn` _playercontroller) _playercontroller)
        (set `PlayerController.bShowMouseCursor` true _playercontroller)))
    (:`Is Not Valid`
      _))
  (`self.SetActorTickEnabled` false)
  (bind _outactor (`LevelSequencePlayer.CreateLevelSequencePlayer` (`self.CinematicSequence`) (make `MovieSceneSequencePlaybackSettings` false (struct) `Play Rate`)))
  ;[1 1 1] Play the cinematic
  (bind _output_get_2 (set `self.SequencePlayerRef` (`LevelSequenceActor.SequencePlayer` _outactor)))
  (`MovieSceneSequencePlayer.Play` _output_get_2)
  (`self.SetActorTickEnabled` true)
  ;[1 1 1] When is finished
  (add `MovieSceneSequencePlayer.OnFinished` _output_get_2 (delegate `API_CinematicFinish`))
  ;[1 1 1] Once the stop
  (add `MovieSceneSequencePlayer.OnStop` _output_get_2 (delegate `API_CinematicStop`)))

(event `CinematicStop`
  (`self.API_StopCinematic`))

(event `CinematicPause or Unpause`
  (`self.API_CinematicTooglePause`))

(event `API_CinematicFinish`
  ;[1 1 1] When is finished
  (`self.API_SpawnCameraSmoothTransitionActor`))

(event `API_CinematicStop`
  ;[1 1 1] Once the stop
  (`self.API_SpawnCameraSmoothTransitionActor`))

(event `self.ReceiveTick`
  (params (DeltaSeconds :type "Float (single-precision)"))
  (bind _sequenceplayerref (`self.SequencePlayerRef`))
  (bind _returnvalue (`LevelSequencePlayer.GetActiveCameraComponent` _sequenceplayerref))
  ;[1 1 1] Get the cinematic last know camera position for the smooth transition
  (`/Engine/EditorBlueprintResources/StandardMacros.IsValid` _sequenceplayerref
    (:`Is Valid`
      (`/Engine/EditorBlueprintResources/StandardMacros.IsValid` _returnvalue
        (:`Is Valid`
          (set `self.LastKnowCameraPosition` (`SceneComponent.K2_GetComponentToWorld` _returnvalue)))))))

(event `API_SpawnCameraSmoothTransitionActor`
  (bind _playercontroller (`self.PlayerController`))
  (bind _cinematiccontrollwidget (`self.CinematicControllWidget`))
  (bind _confirmationmodal (`/Game/MasterRpgFramework/MasterCinematicManager/Widget/WBP_CinematicSkip.ConfirmationModal` _cinematiccontrollwidget))
  ;[1 1 1] Spawn the actor that will do the return smooth camera
  (set `self.CinematicCompleted` true)
  (`Widget.RemoveFromParent` _cinematiccontrollwidget)
  (`/Engine/EditorBlueprintResources/StandardMacros.IsValid` _confirmationmodal
    (:`Is Valid`
      (`Widget.RemoveFromParent` _confirmationmodal))
    (:`Is Not Valid`
      _))
  (if (`self.UseCameraSmoothTransition`)
    (`/Engine/EditorBlueprintResources/StandardMacros.IsValid` (`self.PlayerController`)
      (:`Is Valid`
        (bind _returnvalue (`|SpawnActorFromClass` (`self.ReturnCameraClass`) (`self.LastKnowCameraPosition`) "Undefined" "MultiplyWithRoot" null null))
        (bind _asbp_base_cinematic_to_player_camera (cast `/Game/MasterRpgFramework/MasterCinematicManager/CinematicToPlayer/BP_BaseCinematicToPlayerCamera` _returnvalue))
        (bind _camera (message `/Game/MasterRpgFramework/MasterCinematicManager/CInematicManager/BPI_CinematicManager.I_ReturnCurrentPlayerCamera` (`Controller.K2_GetPawn` _playercontroller)))
        (`/Game/MasterRpgFramework/MasterCinematicManager/CinematicToPlayer/BP_BaseCinematicToPlayerCamera.API_StartTranstion` _asbp_base_cinematic_to_player_camera _playercontroller _camera)
        (add `/Game/MasterRpgFramework/MasterCinematicManager/CinematicToPlayer/BP_BaseCinematicToPlayerCamera.TransitionFinish` _asbp_base_cinematic_to_player_camera (delegate `API_CinematicComplete`))))
    (else
      (`self.API_CinematicComplete`))))

(event `API_CinematicTooglePause`
  (bind _sequenceplayerref (`self.SequencePlayerRef`))
  ;[1 1 1] Handle the pause and unpause of the cinematic
  (if (`MovieSceneSequencePlayer.IsPaused` _sequenceplayerref)
    (`MovieSceneSequencePlayer.Play` _sequenceplayerref)
    (`self.EV_CinematicPlay`)
    (else
      (`MovieSceneSequencePlayer.Pause` _sequenceplayerref)
      (`self.EV_CinematicPause`))))

(event `API_StopCinematic`
  ;[1 1 1] Stop the cinematic from playing
  (`self.EV_CinematicStop`)
  (if (`self.Skipppable`)
    (`MovieSceneSequencePlayer.Stop` (`self.SequencePlayerRef`))))

(event `API_CinematicComplete`
  ;[1 1 1] Spawn the actor that will do the return smooth camera
  (`self.EV_CinematicComplete`)
  (if (or (`self.DestroyOnFinish`) (`self.DestroyOnStop`))
    (`self.K2_DestroyActor`)))

(fn `UserConstructionScript`)